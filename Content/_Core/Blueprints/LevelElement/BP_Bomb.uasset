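; BP_Bomb is a level element that, on its first Hit event, applies a one-time radial force to nearby physics objects and destroys itself.
; A multi-sphere trace on the Visibility channel finds surrounding actors, keeping those whose root component simulates physics.
; The force on each hit component points from that actor toward the bomb, so it pulls objects inward.
; Debug trace drawing and name printing are left on.
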(event Collision|EventHit
  (params (MyComp :type Primitive%20Component%20Object%20Reference) (Other :type Actor%20Object%20Reference) (OtherComp :type Primitive%20Component%20Object%20Reference) (bSelfMoved :type Boolean) (HitLocation :type Vector :default "0, 0, 0") (HitNormal :type Vector :default "0, 0, 0") (NormalImpulse :type Vector :default "0, 0, 0") (Hit :type Hit%20Result%20Structure%20%28by%20ref%29))
  (bind _returnvalue (Transformation|GetActorLocation))
  (Utilities|FlowControl|DoOnce false
    (:Completed
      (bind _outhits (Collision|MultiSphereTraceByChannel _returnvalue _returnvalue 7.5e+02 "TraceTypeQuery1" true 0 "ForDuration"))
      (for _array_element _outhits
        (if (Physics|IsSimulatingPhysics (Variables|/Script/Engine.Actor|GetRootComponent (.HitActor (Collision|BreakHitResult _array_element))) "None")
          (Development|PrintString (Utilities|GetDisplayName (.HitActor (Collision|BreakHitResult _array_element))))
          (Physics|AddForce (.HitComponent (Collision|BreakHitResult _array_element)) (* (Math|Vector|GetForwardVector (Math|Rotator|FindLookatRotation (Transformation|GetActorLocation (.HitActor (Collision|BreakHitResult _array_element))) (Transformation|GetActorLocation))) 5e+07) "None" false)))
      (Actor|DestroyActor))))

(fn ConstructionScript)
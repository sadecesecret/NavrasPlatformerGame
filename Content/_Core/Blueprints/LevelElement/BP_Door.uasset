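; BP_Door is a level element door that swings open when the player's third-person character enters its trigger box, provided CanOpen is set.
; The overlap calls OpenDoor, which plays the DoorRotation timeline to lerp the static mesh's relative rotation toward DoorRotationAngle along the shortest path.
; CloseDoor reverses the same timeline, but nothing in this Blueprint calls it.
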(event OnComponentBeginOverlap(Box)
  (params (OverlappedComponent :type Primitive%20Component%20Object%20Reference) (OtherActor :type Actor%20Object%20Reference) (OtherComp :type Primitive%20Component%20Object%20Reference) (OtherBodyIndex :type Integer) (bFromSweep :type Boolean) (SweepResult :type Hit%20Result%20Structure%20%28by%20ref%29))
  (Utilities|Casting|CastToBP_ThirdPersonCharacter OtherActor)
  (if (Variables|Default|GetCanOpen)
    (CallFunction|OpenDoor)))

(event Custom|OpenDoor
  (bind _dooropenalphavalue (Timeline|DoorRotation Play)
    (:Update
      (Transformation|SetRelativeRotation (Variables|Default|GetStaticMesh) (Math|Rotator|Lerp(Rotator) "0, 0, 0" (Variables|Default|GetDoorRotationAngle) _dooropenalphavalue true) false false))))

(event Custom|CloseDoor
  (bind _dooropenalphavalue (Timeline|DoorRotation Reverse)
    (:Update
      (Transformation|SetRelativeRotation (Variables|Default|GetStaticMesh) (Math|Rotator|Lerp(Rotator) "0, 0, 0" (Variables|Default|GetDoorRotationAngle) _dooropenalphavalue true) false false))))

(event EventBeginPlay)

(fn ConstructionScript)
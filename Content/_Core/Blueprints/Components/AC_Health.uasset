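; AC_Health is a health component that tracks current health and alive state for its owner.
; GainHealth and GainDamage adjust CurrentHealth, clamped between zero and MaxHealth, with healing firing the OnHealth dispatcher.
; Damage also updates IsAlive, then fires OnGainDamage while health remains or calls Died, which broadcasts OnDied.
; The event graph holds only an empty custom event and unconnected calls.
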(event Custom|MyCustom%20Event)

(fn GainHealth
  (params (HealthAmount :type Integer))
  (Variables|Default|SetCurrentHealth (Math|Integer|Clamp(Integer) (+ (Variables|Default|GetCurrentHealth) HealthAmount) 0 (Variables|Default|GetMaxHealth)))
  (Default|CallOnHealth)
  (return (Variables|Default|GetCurrentHealth)))

(fn GainDamage
  (params (DamageAmount :type Integer))
  (Variables|Default|SetCurrentHealth (Math|Integer|Clamp(Integer) (- (Variables|Default|GetCurrentHealth) DamageAmount) 0 (Variables|Default|GetMaxHealth)))
  (bind _output_get (Variables|Default|SetIs%20Alive (> (Variables|Default|GetCurrentHealth) 0)))
  (if _output_get
    (Default|CallOnGainDamage)
    (return (Variables|Default|GetIs%20Alive))
    (else
      (CallFunction|Died))))

(fn Died
  (Default|CallOnDied))
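; BP_platform is a moving platform that rises once any actor overlaps it.
; It records its location on BeginPlay, and an overlap sets CanMove.
; While CanMove is set, Tick adds a fixed upward step without sweep or delta-time scaling, so speed follows frame rate.
; Movement stops when the location nearly equals StartPos plus Offset, with no return logic.
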(event EventBeginPlay
  ;[1 1 1] Start Position Set
  (Variables|Default|SetStartPos (Transformation|GetActorLocation)))

(event Collision|EventActorBeginOverlap
  (params (OtherActor :type Actor%20Object%20Reference))
  ;[1 1 1] Can move When Overlap begin
  (Variables|Default|SetCanMove true))

(event EventTick
  (params (DeltaSeconds :type Float%20%28single-precision%29))
  ;[1 1 1] Movement and movement control
  (if (Variables|Default|GetCanMove)
    (Transformation|AddActorWorldOffset "0, 0,1.000000")
    (if (Utilities|Operators|EqualEqual (+ (Variables|Default|GetStartPos) (Variables|Default|GetOffset)) (Transformation|GetActorLocation) 5.0)
      (Variables|Default|SetCanMove false))))

(fn ConstructionScript)
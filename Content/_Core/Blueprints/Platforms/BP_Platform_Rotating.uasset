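; Rotating platform actor that starts turning when play begins and can optionally swing back and forth.
; A timeline at a configurable play rate lerps the Scene component's relative rotation from zero to the target RotatingDegree.
; When looping is enabled, each finish waits a tick, then a FlipFlop alternates between reversing and replaying the timeline.
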(event Custom|PlayAnimation
  ;[1 1 1] Rotating animation
  (bind _movement_alpha (Timeline|Platfrom%20Movement Play)
    (:Update
      (Transformation|SetRelativeRotation (Variables|Default|GetScene) (Math|Rotator|Lerp(Rotator) "0, 0, 0" (Variables|Default|GetRotatingDegree) _movement_alpha) false false))
    (:Finished
      (Utilities|FlowControl|DelayUntilNextTick)
      (if (Variables|Default|GetIsLooping)
        (Utilities|FlowControl|FlipFlop
          (:A
            (CallFunction|PlayReverseAnimation))
          (:B
            (CallFunction|PlayAnimation)))))))

(event Custom|PlayReverseAnimation
  ;[1 1 1] Rotating animation
  (bind _movement_alpha (Timeline|Platfrom%20Movement Reverse)
    (:Update
      (Transformation|SetRelativeRotation (Variables|Default|GetScene) (Math|Rotator|Lerp(Rotator) "0, 0, 0" (Variables|Default|GetRotatingDegree) _movement_alpha) false false))
    (:Finished
      (Utilities|FlowControl|DelayUntilNextTick)
      (if (Variables|Default|GetIsLooping)
        (Utilities|FlowControl|FlipFlop
          (:A
            (CallFunction|PlayReverseAnimation))
          (:B
            (CallFunction|PlayAnimation)))))))

(event EventBeginPlay
  ;[1 1 1] Start Position Set
  (Components|Timeline|SetPlayRate (Variables|Default|GetPlatfrom%20Movement%20) (Variables|Default|GetPlayRate))
  (Components|Timeline|PlayfromStart (Variables|Default|GetPlatfrom%20Movement%20)))

(fn ConstructionScript)
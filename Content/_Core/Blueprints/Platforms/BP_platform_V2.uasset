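; BP_platform_V2 is a moving platform that travels from its placed position by an offset when play begins.
; BeginPlay stores the start location and plays a timeline whose alpha lerps the actor to start plus offset, without sweep.
; The timeline's finish only delays a tick, and the FlipFlop meant to alternate reverse and play is never triggered.
; Overlap and Tick events are empty.
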(event EventBeginPlay
  ;[1 1 1] Start Position Set
  (Variables|Default|SetStartLocation (Transformation|GetActorLocation))
  (Components|Timeline|PlayfromStart (Variables|Default|GetPlatfrom%20Movement%20)))

(event Collision|EventActorBeginOverlap
  (params (OtherActor :type Actor%20Object%20Reference))
  ;[1 1 1] Can move When Overlap begin
)

(event EventTick
  (params (DeltaSeconds :type Float%20%28single-precision%29))
  ;[1 1 1] Movement and movement control
)

(fn ConstructionScript)
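; BP_Projectile is a trap projectile actor that explodes on impact and damages whatever it hits.
; On a sphere collision hit it spawns a Niagara explosion at the impact point, applies fixed damage through the hit actor's AC_Health component if present, then destroys itself.
; The construction script copies exposed gravity scale, initial speed and bounce settings into its ProjectileMovement component.
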(event OnComponentHit(SphereCol)
  (params (HitComponent :type Primitive%20Component%20Object%20Reference) (OtherActor :type Actor%20Object%20Reference) (OtherComp :type Primitive%20Component%20Object%20Reference) (NormalImpulse :type Vector :default "0, 0, 0") (Hit :type Hit%20Result%20Structure%20%28by%20ref%29))
  (Variables|Default|SetHitActor OtherActor)
  (CallFunction|PlayVFX (.Location (Collision|BreakHitResult Hit)))
  (Utilities|FlowControl|Sequence
    (:then_0
      (Utilities|IsValid (Actor|GetComponentbyClass (Variables|Default|GetHitActor) "/Game/_Core/Blueprints/Components/AC_Health.AC_Health_C")
        (:Is%20Valid
          (Default|GainDamage (Actor|GetComponentbyClass (Variables|Default|GetHitActor) "/Game/_Core/Blueprints/Components/AC_Health.AC_Health_C") 50))))
    (:then_1
      (Actor|DestroyActor))))

(event Custom|PlayVFX
  (params (Location :type Vector))
  (Niagara|SpawnSystematLocation "/Game/sA_Megapack_v1/sA_StylizedAttacksPack/FX/NiagaraSystems/NS_AOE_Explosion_1.NS_AOE_Explosion_1" Location))

(fn ConstructionScript
  (Variables|/Script/Engine.ProjectileMovementComponent|SetProjectileGravityScale (Variables|Default|GetProjectileMovement) (Variables|Default|GetProjectile%20Gravity%20Scale))
  (Variables|/Script/Engine.ProjectileMovementComponent|SetInitialSpeed (Variables|Default|GetProjectileMovement) (Variables|Default|GetInitial%20Speed))
  (Variables|/Script/Engine.ProjectileMovementComponent|SetbShouldBounce (Variables|Default|GetProjectileMovement) (Variables|Default|GetShould%20Bounce)))
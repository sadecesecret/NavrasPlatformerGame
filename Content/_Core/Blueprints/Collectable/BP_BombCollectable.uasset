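; BP_BombCollectable is a collectable pickup that gives the player a bomb.
; On first interaction it allows interaction only if the player has no valid Bomb.
; When collected it rechecks that reference and calls SpawnBomb on the player, or prints a debug string if a bomb already exists.
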(event EventBeginPlay
  (|CallParentFunction) ; This node is disabled and will not be called.\nDrag off pins to build functionality.
)

(event EventCollected
  (Utilities|IsValid (Variables|/Game/_Core/Blueprints/Characters/BP_ThirdPersonCharacter.BP_ThirdPersonCharacter_C|GetBomb (Variables|Default|GetPlayerRef))
    (:Is%20Valid
      (Development|PrintString "Valid Object "))
    (:Is%20Not%20Valid
      (Default|SpawnBomb (Variables|Default|GetPlayerRef)))))

(event EventFirstInteraction
  (Variables|Default|SetCanInteract (not (Utilities|IsValid (Variables|/Game/_Core/Blueprints/Characters/BP_ThirdPersonCharacter.BP_ThirdPersonCharacter_C|GetBomb (Variables|Default|GetPlayerRef))))))

(fn ConstructionScript
  (|CallParentFunction))
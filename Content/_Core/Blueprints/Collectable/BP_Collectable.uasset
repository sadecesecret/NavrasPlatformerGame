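; BP_Collectable is a pickup actor that the third-person player character collects by touching it.
; On the first sphere overlap with that character, a DoOnce hides the mesh, calls Collected, plays a sound at the actor's location and adds a Niagara effect component.
; Collected is an empty event, and the actor is hidden rather than destroyed.
; BeginPlay caches a player reference that this graph does not otherwise use.
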(event OnComponentBeginOverlap(Sphere)
  (params (OverlappedComponent :type Primitive%20Component%20Object%20Reference) (OtherActor :type Actor%20Object%20Reference) (OtherComp :type Primitive%20Component%20Object%20Reference) (OtherBodyIndex :type Integer) (bFromSweep :type Boolean) (SweepResult :type Hit%20Result%20Structure%20%28by%20ref%29))
  (Utilities|Casting|CastToBP_ThirdPersonCharacter OtherActor)
  (Utilities|FlowControl|DoOnce false
    (:Completed
      (Rendering|SetVisibility (Variables|Default|GetStaticMesh) false true)
      (CallFunction|Collected)
      (CallFunction|PlayAudio)
      (CallFunction|PlayVFX))))

(event Custom|Collected)

(event Custom|Play%20Audio
  (Audio|PlaySoundatLocation (Variables|Default|GetSound) (Transformation|GetActorLocation) "0, 0, 0" 1.0 1.0 0.0 0 0 0 0))

(event Custom|PlayVFX
  (bind _returnvalue (AddComponent|AddNiagaraComponent false))
  (Variables|Default|SetVFX _returnvalue)
  (Class|NiagaraComponent|SetAsset (Variables|Default|GetVFX) (Variables|Default|GetVFX%20Asset) true))

(event EventBeginPlay
  (bind _asbp_third_person_character (Utilities|Casting|CastToBP_ThirdPersonCharacter (Game|Player|GetPlayerPawn 0)))
  (Variables|Default|SetPlayerRef _asbp_third_person_character))

(fn ConstructionScript)